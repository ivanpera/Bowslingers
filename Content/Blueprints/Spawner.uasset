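; Spawner actor that spawns a given actor class at its own location, optionally randomized per axis within its Box component's bounds.
; The SpawnActor event passes the class and SpawnConfig to SpawnActorHandle, which validates the class and loops over the XYZ config entries.
; Axes flagged Randomize take a coordinate from a random point in the box, while others keep the spawner's coordinate.
; Spawning always succeeds regardless of collision.
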(event EventSpawnActor
  (params (SpawnConfig :type Spawn%20Config%20Structure%20%28by%20ref%29) (ActorClass :type Actor%20Class%20Reference))
  (CallFunction|SpawnActorHandle SpawnConfig ActorClass))

(fn ConstructionScript)

(fn SpawnActorHandle
  (params (SpawnConfig :type Spawn%20Config%20Structure) (Actor :type Actor%20Class%20Reference))
  (bind _returnvalue (Transformation|GetActorLocation))
  (bind _box (Variables|Default|GetBox))
  (bind (_origin _boxextent) (Collision|GetComponentBounds _box))
  (bind _returnvalue_2 (Math|Random|RandomPointinBoundingBox _origin _boxextent))
  (if (Utilities|IsValidClass Actor)
    (bind _output_get (LocalVariables|SetActorLocation (Utilities|Array|MakeArray (.x _returnvalue) (.y _returnvalue) (.z _returnvalue))))
    (LocalVariables|SetSpawnLocation _output_get)
    (for (_array_element _array_index) (.xyzconfig SpawnConfig)
      (LocalVariables|SetIdx _array_index)
      (if (.randomize _array_element)
        (if (.bound _array_element)
          _
          (else
            _))
        (Utilities|Array|SetArrayElem (LocalVariables|GetSpawnLocation) (LocalVariables|GetIdx) (Utilities|Array|Get(acopy) (Utilities|Array|MakeArray (.x _returnvalue_2) (.y _returnvalue_2) (.z _returnvalue_2)) (LocalVariables|GetIdx)))
        (else
          (Utilities|Array|SetArrayElem (LocalVariables|GetSpawnLocation) (LocalVariables|GetIdx) (Utilities|Array|Get(acopy) (LocalVariables|GetActorLocation) _array_index)))))
    (Game|SpawnActorfromClass Actor (Math|Transform|MakeTransform (Math|Vector|MakeVector (Utilities|Array|Get(acopy) (LocalVariables|GetSpawnLocation)) (Utilities|Array|Get(acopy) (LocalVariables|GetSpawnLocation) 1) (Utilities|Array|Get(acopy) (LocalVariables|GetSpawnLocation) 2)) "0, 0, 0" "1,1,1") "AlwaysSpawn" 0 0)))