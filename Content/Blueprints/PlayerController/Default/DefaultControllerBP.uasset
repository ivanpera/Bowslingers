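; Player controller for a turn-based bow game that turns a mouse drag into an arrow shot from the BowmanBP pawn.
; DrawBow input drives an idle, drawing, loose state machine on Tick, with drag length capped relative to viewport size to set power and direction.
; On release, it fires the bowman's arrow if CanShoot, while ReloadArrow attaches new arrows to the hand socket.
; Tick blocks input when the GameState's current bowman differs from the pawn.
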(event EventBeginPlay
  (Variables|Default|SetbShowMouseCursor true)
  (Variables|Default|SetIgnoreInput false)
  (Variables|Default|SetInputState "NewEnumerator0"))

(event EventTick
  (params (DeltaSeconds :type Float%20%28single-precision%29))
  (bind _currentbowman (Default|GetCurrentBowman (.AsDefault%20Game%20State%20BP (Utilities|Casting|CastToDefaultGameStateBP (Game|GetGameState)))))
  (if (!= _currentbowman (Game|Player|GetPlayerPawn 0))
    (Variables|Default|SetIgnoreInput true))
  (switch Utilities|FlowControl|Switch|SwitchonEControllerState (Variables|Default|GetInputState)
    (:NewEnumerator1
      (if (not (Variables|Default|GetIgnoreInput))
        (Variables|Default|SetMaxDragLength (* (Math|Vector2D|Vector2DLength (Viewport|GetViewportSize)) 0.3))
        (CallFunction|UpdateCurrDrawPosition)
        (CallFunction|UpdateDrawPower)))
    (:NewEnumerator2
      (if (Variables|Default|GetCanShoot)
        (CallFunction|ShootArrow)))))

(event Input|ActionEvents|InputActionDrawBow
  (params (Key :type Key%20Structure))
  (bind (_locationx _locationy) (Game|Player|GetMousePosition))
  (:Pressed
    (if (not (Variables|Default|GetIgnoreInput))
      (if (Utilities|Enum|Equal(Enum) (Variables|Default|GetInputState) "NewEnumerator0")
        (bind _output_get (Variables|Default|SetStartDragPosition (Math|Vector2D|MakeVector2D _locationx _locationy)))
        (Variables|Default|SetCurrDragPosition _output_get)
        (Variables|Default|SetInputState "NewEnumerator1"))))
  (:Released
    (if (Utilities|Enum|Equal(Enum) (Variables|Default|GetInputState) "NewEnumerator1")
      (Variables|Default|SetInputState "NewEnumerator2"))))

(fn ConstructionScript)

(fn ShootArrow
  (bind _returnvalue (Game|Player|GetPlayerPawn 0))
  (bind _asbowman_bp (Utilities|Casting|CastToBowmanBP _returnvalue))
  (bind _arrow (Variables|/Game/Blueprints/Bowman/BowmanBP.BowmanBP_C|GetArrow _asbowman_bp))
  (Utilities|IsValid _arrow
    (:Is%20Valid
      (bind _asarrow_bp (Utilities|Casting|CastToArrow_BP _arrow))
      (Default|ShootArrow _asarrow_bp (Variables|Default|GetDrawPower) (Variables|Default|GetDragDirection))
      (Variables|Default|SetInputState "NewEnumerator0"))))

(fn UpdateCurrDrawPosition
  (bind (_locationx _locationy) (Game|Player|GetMousePosition))
  (bind _startdragposition (Variables|Default|GetStartDragPosition))
  (bind _maxdraglength (Variables|Default|GetMaxDragLength))
  (bind _returnvalue (Math|Vector2D|MakeVector2D _locationx _locationy))
  (bind _returnvalue_2 (- _returnvalue _startdragposition))
  (bind _returnvalue_3 (Math|Vector2D|Vector2DLength _returnvalue_2))
  (bind _returnvalue_4 (Math|Vector2D|Normalize2D _returnvalue_2))
  (bind _returnvalue_5 (Math|Float|Min(Float) _maxdraglength _returnvalue_3))
  (bind _returnvalue_6 (* _returnvalue_4 _returnvalue_5))
  (Variables|Default|SetCurrDragPosition (+ (Variables|Default|GetStartDragPosition) _returnvalue_6))
  (Variables|Default|SetDragDirection (Math|Vector2D|Normalize2D _returnvalue_6)))

(fn UpdateDrawPower
  (Variables|Default|SetDrawPower (/ (Math|Vector2D|Vector2DLength (- (Variables|Default|GetCurrDragPosition) (Variables|Default|GetStartDragPosition))) (Variables|Default|GetMaxDragLength))))

(fn ReloadArrow
  (bind _returnvalue (Game|Player|GetPlayerPawn 0))
  (bind _asbowman_bp (Utilities|Casting|CastToBowmanBP _returnvalue))
  (bind _returnvalue_2 (Game|SpawnActorfromClass "/Game/Blueprints/Arrows/Arrow_BP.Arrow_BP_C" (Math|Transform|MakeTransform "0, 0, 0" "0, 0, 0" "1,1,1") "AlwaysSpawn" (Game|Player|GetPlayerPawn 0) 0))
  (bind _output_get (Variables|/Game/Blueprints/Bowman/BowmanBP.BowmanBP_C|SetArrow _asbowman_bp _returnvalue_2))
  (Transformation|AttachComponentToComponent _output_get (Variables|/Game/Blueprints/Bowman/BowmanBP.BowmanBP_C|GetSkeletalMesh _asbowman_bp) "RightHandSocket" "SnapToTarget" "SnapToTarget" "SnapToTarget" false))