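; Game mode for a turn-based archery game in which one player controller possesses each bowman in turn.
; On BeginPlay it creates the HUD, stores all bowmen in the game state and spawns a shared follow camera.
; A shot makes the camera follow the arrow and blocks input.
; A hit advances the bowman index, then a one-second timer retargets the camera, possesses the next bowman and restores input.
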(event Custom|OnArrowShot
  (params (Arrow :type Actor%20Object%20Reference))
  (CallFunction|HandleArrowShot Arrow))

(event Custom|OnArrowHit
  (params (Arrow :type Actor%20Object%20Reference))
  (CallFunction|HandleArrowHit Arrow))

(event EventBeginPlay
  (bind _returnvalue (Game|GetPlayerController 0))
  (bind _returnvalue_2 (UserInterface|CreateWidget "/Game/Blueprints/HUD.HUD_C" _returnvalue))
  (UserInterface|Viewport|AddtoPlayerScreen _returnvalue_2)
  (CallFunction|SetUpGame)
  (Input|SetInputModeGameandUI _returnvalue 0 "DoNotLock" false))

(fn ConstructionScript)

(fn SetUpGame
  (bind _asdefault_game_state_bp (Utilities|Casting|CastToDefaultGameStateBP (Game|GetGameState)))
  (Utilities|FlowControl|Sequence
    (:then_0
      (Variables|/Game/Blueprints/GameStates/DefaultGameStateBP.DefaultGameStateBP_C|SetMatchState _asdefault_game_state_bp "NewEnumerator1"))
    (:then_1
      (bind _outactors (Actor|GetAllActorsOfClass "/Game/Blueprints/Bowman/BowmanBP.BowmanBP_C"))
      (bind _output_get (Variables|/Game/Blueprints/GameStates/DefaultGameStateBP.DefaultGameStateBP_C|SetBowmen _asdefault_game_state_bp _outactors)))
    (:then_2
      (bind _output_get_2 (Variables|/Game/Blueprints/GameStates/DefaultGameStateBP.DefaultGameStateBP_C|SetCurrentBowmanIdx _asdefault_game_state_bp 0))
      (Pawn|Possess (Game|GetPlayerController 0) (Utilities|Array|Get(acopy) _output_get _output_get_2)))
    (:then_3
      (CallFunction|SetMainCamera))))

(fn HandleArrowShot
  (params (Arrow :type Actor%20Object%20Reference))
  (Class|FollowTargetComponent|SetTargetandTime (Variables|/Game/Blueprints/FollowCameraBP.FollowCameraBP_C|GetFollowTarget (Variables|/Game/Blueprints/GameStates/DefaultGameStateBP.DefaultGameStateBP_C|GetMainCamera (.AsDefault%20Game%20State%20BP (Utilities|Casting|CastToDefaultGameStateBP (Game|GetGameState))))) Arrow 0.05)
  (Variables|/Game/Blueprints/PlayerController/Default/DefaultControllerBP.DefaultControllerBP_C|SetIgnoreInput (.AsDefault%20Controller%20BP (Utilities|Casting|CastToDefaultControllerBP (Game|GetPlayerController 0))) true))

(fn HandleArrowHit
  (params (Arrow :type Actor%20Object%20Reference))
  (bind _returnvalue (Game|GetGameState))
  (bind _asdefault_game_state_bp (Utilities|Casting|CastToDefaultGameStateBP _returnvalue))
  (Variables|/Game/Blueprints/GameStates/DefaultGameStateBP.DefaultGameStateBP_C|SetCurrentBowmanIdx _asdefault_game_state_bp (Math|Integer|%(Integer) (+ (Variables|/Game/Blueprints/GameStates/DefaultGameStateBP.DefaultGameStateBP_C|GetCurrentBowmanIdx _asdefault_game_state_bp) 1) (Utilities|Array|Length (Variables|/Game/Blueprints/GameStates/DefaultGameStateBP.DefaultGameStateBP_C|GetBowmen _asdefault_game_state_bp))))
  (Utilities|Time|SetTimerbyFunctionName self "DisposeArrow" 1.0))

(fn DisposeArrow
  (bind _returnvalue (Game|GetGameState))
  (bind _returnvalue_2 (Game|GetPlayerController 0))
  (bind _asdefault_controller_bp (Utilities|Casting|CastToDefaultControllerBP _returnvalue_2))
  (bind _asdefault_game_state_bp (Utilities|Casting|CastToDefaultGameStateBP _returnvalue))
  (bind _currentbowman (Default|GetCurrentBowman _asdefault_game_state_bp))
  (Class|FollowTargetComponent|SetTargetandTime (Variables|/Game/Blueprints/FollowCameraBP.FollowCameraBP_C|GetFollowTarget (Variables|/Game/Blueprints/GameStates/DefaultGameStateBP.DefaultGameStateBP_C|GetMainCamera _asdefault_game_state_bp)) _currentbowman 0.25)
  (Pawn|Possess _asdefault_controller_bp _currentbowman)
  (Variables|/Game/Blueprints/PlayerController/Default/DefaultControllerBP.DefaultControllerBP_C|SetIgnoreInput _asdefault_controller_bp false))

(fn SetMainCamera
  (bind _returnvalue (Game|GetGameState))
  (bind _asdefault_game_state_bp (Utilities|Casting|CastToDefaultGameStateBP _returnvalue))
  (bind _returnvalue_2 (Game|SpawnActorfromClass "/Game/Blueprints/FollowCameraBP.FollowCameraBP_C" (Math|Transform|MakeTransform "0, 0, 0" "0, 0, 0" "1,1,1") "AlwaysSpawn" 0 0))
  (bind _output_get (Variables|/Game/Blueprints/GameStates/DefaultGameStateBP.DefaultGameStateBP_C|SetMainCamera _asdefault_game_state_bp _returnvalue_2))
  (Utilities|FlowControl|Sequence
    (:then_0
      (Class|FollowTargetComponent|SetTargetandTime (Variables|/Game/Blueprints/FollowCameraBP.FollowCameraBP_C|GetFollowTarget _output_get) (Utilities|Array|Get(acopy) (Variables|/Game/Blueprints/GameStates/DefaultGameStateBP.DefaultGameStateBP_C|GetBowmen _asdefault_game_state_bp) (Variables|/Game/Blueprints/GameStates/DefaultGameStateBP.DefaultGameStateBP_C|GetCurrentBowmanIdx _asdefault_game_state_bp)) 0.0)
      (EventDispatchers|BindEventtoOnSnap (Variables|/Game/Blueprints/FollowCameraBP.FollowCameraBP_C|GetFollowTarget _output_get) (EventDispatchers|CreateEvent self :!event HandleCameraSnap))
      (Variables|/Script/Bowman.FollowTargetComponent|SetOffset (Variables|/Game/Blueprints/FollowCameraBP.FollowCameraBP_C|GetFollowTarget _output_get) "-200.000000,0.000000, 0"))
    (:then_1
      (Game|Player|SetViewTargetwithBlend (Game|GetPlayerController 0) _output_get 0.0 "VTBlend_Linear" 0.0 false))))

(fn HandleCameraSnap
  (bind _returnvalue (Game|GetGameState))
  (bind _asdefault_game_state_bp (Utilities|Casting|CastToDefaultGameStateBP _returnvalue))
  (bind _maincamera (Variables|/Game/Blueprints/GameStates/DefaultGameStateBP.DefaultGameStateBP_C|GetMainCamera _asdefault_game_state_bp))
  (bind _followtarget (Variables|/Game/Blueprints/FollowCameraBP.FollowCameraBP_C|GetFollowTarget _maincamera))
  (bind _target (Variables|/Script/Bowman.FollowTargetComponent|GetTarget _followtarget))
  (Utilities|IsValid _target
    (:Is%20Valid
      (Utilities|Casting|CastToBowmanBP _target)
      (Variables|/Game/Blueprints/PlayerController/Default/DefaultControllerBP.DefaultControllerBP_C|SetIgnoreInput (.AsDefault%20Controller%20BP (Utilities|Casting|CastToDefaultControllerBP (Game|GetPlayerController 0))) false))))