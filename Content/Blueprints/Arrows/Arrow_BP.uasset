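; Arrow projectile actor that is fired from its owner and sticks into what it hits, notifying DefaultGameModeBP of shots and hits.
; ShootArrow detaches it, adds a ProjectileMovement component at runtime with velocity from draw power and drag direction, and enables collision.
; Valid overlaps destroy that component, disable collision and attach the arrow at a randomized depth to the hit component or bone.
; Validation rejects boneless skeletal-mesh hits, itself, and its owner during a post-shot grace period.
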(event OnComponentBeginOverlap(StaticMesh)
  (params (OverlappedComponent :type Primitive%20Component%20Object%20Reference) (OtherActor :type Actor%20Object%20Reference) (OtherComp :type Primitive%20Component%20Object%20Reference) (OtherBodyIndex :type Integer) (bFromSweep :type Boolean) (SweepResult :type Hit%20Result%20Structure%20%28by%20ref%29))
  (bind _shouldhandle (CallFunction|HandleOverlap SweepResult))
  (if _shouldhandle
    (Default|OnArrowHit (.AsDefault%20Game%20Mode%20BP (Utilities|Casting|CastToDefaultGameModeBP (Game|GetGameMode))) self)))

(fn ConstructionScript)

(fn ShootArrow
  (params (DrawPower :type Float%20%28single-precision%29) (DragDirection :type Vector%202D%20Structure))
  (bind _returnvalue (Transformation|GetActorRotation))
  (bind _returnvalue_2 (Components|GetOwner))
  (Transformation|SetActorRotation (Math|Rotator|MakeRotator (.roll _returnvalue) (.pitch _returnvalue) (.yaw (Transformation|GetActorRotation (Components|GetOwner)))))
  (Transformation|DetachFromActor "KeepWorld" "KeepWorld" "KeepWorld")
  (bind _returnvalue_3 (AddComponent|AddProjectileMovementComponent))
  (Variables|Default|SetProjectileMovement _returnvalue_3)
  (Utilities|FlowControl|Sequence
    (:then_0
      (Variables|/Script/Engine.ProjectileMovementComponent|SetbRotationFollowsVelocity (Variables|Default|GetProjectileMovement) true))
    (:then_1
      (Variables|/Script/Engine.MovementComponent|SetVelocity (Variables|Default|GetProjectileMovement) (* (+ (* (Transformation|GetActorForwardVector _returnvalue_2) (Math|Float|Absolute(Float) (.x DragDirection))) (* (Transformation|GetActorUpVector _returnvalue_2) (.y DragDirection))) (* (Variables|Default|GetInitialSpeed) DrawPower)))
      (Variables|Default|SetTimeOfShooting (Math|DateTime|UTCNow)))
    (:then_2
      (Default|OnArrowShot (.AsDefault%20Game%20Mode%20BP (Utilities|Casting|CastToDefaultGameModeBP (Game|GetGameMode))) self)
      (Collision|SetCollisionEnabled (Variables|Default|GetStaticMesh) "QueryAndPhysics"))))

(fn HandleOverlap
  (params (HitResult :type Hit%20Result%20Structure%20%28by%20ref%29))
  (bind _projectilemovement (Variables|Default|GetProjectileMovement))
  (bind _isvalid (CallFunction|IsOverlapValid HitResult))
  (if _isvalid
    (Utilities|IsValid _projectilemovement
      (:Is%20Valid
        (Components|DestroyComponent _projectilemovement)
        (Collision|SetCollisionEnabled (Variables|Default|GetStaticMesh) "NoCollision")
        (Transformation|SetActorLocation (+ (.location HitResult) (* (Transformation|GetActorForwardVector) (* (.y (.BoxExtent (Collision|GetComponentBounds (Variables|Default|GetStaticMesh)))) (Math|Random|RandomFloatinRange 0.3 1.0)))) false true)
        (Transformation|AttachComponentToComponent (.hitcomponent HitResult) (.hitbonename HitResult) "KeepWorld" "KeepWorld" "KeepWorld" true)
        (return true)))))

(fn IsOverlapValid
  (params (HitResult :type Hit%20Result%20Structure))
  (bind _bsuccess (Utilities|Casting|CastToSkeletalMeshComponent (.hitcomponent HitResult)))
  (if (or (and (Utilities|Name|NotEqual(Name) "None" (.hitbonename HitResult)) _bsuccess) (not _bsuccess))
    (if (and (or (>= (Math|Float|Truncate (Class|KismetMathLibrary|GetTotalMilliseconds (- (Math|DateTime|UTCNow) (Variables|Default|GetTimeOfShooting)))) (Variables|Default|GetGracePeriodMs)) (!= (.hitactor HitResult) (Components|GetOwner))) (!= (.hitactor HitResult) self))
      (return true)
      (else
        _)))
  (return false))